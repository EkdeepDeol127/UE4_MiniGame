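; BossBullet is a short-lived projectile actor fired by Boss_Character.
; On BeginPlay it casts its owner to Boss_Character and applies a physics impulse to its Cube along positive or negative Y, based on the boss's ShootDirection flag.
; It destroys itself after a one-second lifetime, or shortly after overlapping an actor tagged Player, with no damage applied in this Blueprint.
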(event `self.ReceiveBeginPlay`
  (bind _cube (`self.Cube`))
  ;[1 1 1] Adds Velocity based on the shooting direction of player and also destroys itself if 1 duration passed or hits an enemy
  (bind _asboss_character (cast `/Game/Assets/Enemy_Boss/Boss_Character` (`self.GetOwner`))
    (:`then`
      (if (`/Game/Assets/Enemy_Boss/Boss_Character.ShootDirection` _asboss_character)
        (`PrimitiveComponent.AddImpulse` _cube (0.0 1000.0 0.0) "None" false)
        (else
          (`PrimitiveComponent.AddImpulse` _cube (0.0 -1000.0 0.0) "None" false)))
      (`KismetSystemLibrary.Delay` 1.0)
      (`self.K2_DestroyActor` :!label _label))
    (:`CastFailed`
      (`KismetSystemLibrary.PrintString` "BossBullet failed to cast"))))

(event `self.ReceiveActorBeginOverlap`
  (params (OtherActor :type "Actor Object Reference"))
  ;[1 1 1] Adds Velocity based on the shooting direction of player and also destroys itself if 1 duration passed or hits an enemy
  (if (`self.ActorHasTag` OtherActor "Player")
    (`KismetSystemLibrary.Delay` 0.05)
    (goto _label)))

(fn `UserConstructionScript`)