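; EnemyRobotBullet is a projectile actor for the Enemy_Robot that destroys itself on reaching the player or timing out.
; On BeginPlay it casts its owner to Enemy_Robot and uses ShootDirection to apply a physics impulse to its Cube along positive or negative Y.
; It is destroyed after a short lifetime, or after a brief delay when it overlaps a Player-tagged actor; no damage is applied here.
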(event `self.ReceiveBeginPlay`
  (bind _cube (`self.Cube`))
  ;[1 1 1] Adds Velocity based on the shooting direction of player and also destroys itself if 1 duration passed or hits an enemy
  (bind _asenemy_robot (cast `/Game/Assets/Enemy_Robot/Enemy_Robot` (`self.GetOwner`))
    (:`then`
      (if (`/Game/Assets/Enemy_Robot/Enemy_Robot.ShootDirection` _asenemy_robot)
        (`PrimitiveComponent.AddImpulse` _cube (0.0 1000.0 0.0) "None" false)
        (else
          (`PrimitiveComponent.AddImpulse` _cube (0.0 -1000.0 0.0) "None" false)))
      (`KismetSystemLibrary.Delay` 1.0)
      (`self.K2_DestroyActor` :!label _label))
    (:`CastFailed`
      (`KismetSystemLibrary.PrintString` "RobotBullet failed to cast"))))

(event `self.ReceiveActorBeginOverlap`
  (params (OtherActor :type "Actor Object Reference"))
  ;[1 1 1] Adds Velocity based on the shooting direction of player and also destroys itself if 1 duration passed or hits an enemy
  (if (`self.ActorHasTag` OtherActor "Player")
    (`KismetSystemLibrary.Delay` 0.05)
    (goto _label)))

(fn `UserConstructionScript`)