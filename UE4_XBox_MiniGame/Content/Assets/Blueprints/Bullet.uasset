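; Bullet is a projectile actor fired by the player character that flies sideways and disappears on a timer or on hitting an enemy.
; On BeginPlay it casts its owner to MainCharacter and applies a Y-axis impulse to its sphere, signed by the shoot direction, then destroys itself after a short lifetime.
; Overlapping an actor tagged as armor enemy, robot enemy or boss destroys it after a brief delay, without applying damage here.
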(event `self.ReceiveBeginPlay`
  (bind _sphere (`self.Sphere`))
  ;[1 1 1] Adds Velocity based on the shooting direction of player and also destroys itself if 1 duration passed or hits an enemy
  (bind _asmain_character (cast `/Game/Assets/MyCharacter/MainCharacter` (`self.GetOwner`))
    (:`then`
      (if (`/Game/Assets/MyCharacter/MainCharacter.ShootDirection` _asmain_character)
        (`PrimitiveComponent.AddImpulse` _sphere (0.0 1000.0 0.0) "None" false)
        (else
          (`PrimitiveComponent.AddImpulse` _sphere (0.0 -1000.0 0.0) "None" false)))
      (`KismetSystemLibrary.Delay` 1.0)
      (`self.K2_DestroyActor` :!label _label))
    (:`CastFailed`
      (`KismetSystemLibrary.PrintString` "Bullet failed to cast"))))

(event `self.ReceiveActorBeginOverlap`
  (params (OtherActor :type "Actor Object Reference"))
  ;[1 1 1] Adds Velocity based on the shooting direction of player and also destroys itself if 1 duration passed or hits an enemy
  (`|ExecutionSequence`
    (:`then_0`
      (if (`self.ActorHasTag` OtherActor "ArmorEnemy")
        (`KismetSystemLibrary.Delay` 0.05 :!label _label_2)
        (goto _label)))
    (:`then_1`
      (if (`self.ActorHasTag` OtherActor "RobotEnemy")
        (goto _label_2)))
    (:`then_2`
      (if (`self.ActorHasTag` OtherActor "Boss")
        (goto _label_2)))))

(fn `UserConstructionScript`)